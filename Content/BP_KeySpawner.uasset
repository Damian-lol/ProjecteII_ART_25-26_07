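; BP_KeySpawner is a trigger actor that spawns a key (Llave1) when the player's laser light hits it.
; On box begin overlap, it checks that the overlapping component is the BP_Khris_LightMechanic player's LightCollision and that LaserLight is visible.
; A DoOnce with no reset limits it to one key, spawned at KeySpawnPoint regardless of collision.
; The end-overlap handler performs a comparison but takes no action.
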(event OnComponentBeginOverlap(Box_collision)
  (params (OverlappedComponent :type Primitive%20Component%20Object%20Reference) (OtherActor :type Actor%20Object%20Reference) (OtherComp :type Primitive%20Component%20Object%20Reference) (OtherBodyIndex :type Integer) (bFromSweep :type Boolean) (SweepResult :type Hit%20Result%20Structure%20%28by%20ref%29))
  (bind _asbp_khris_light_mechanic (Utilities|Casting|CastToBP_Khris_LightMechanic (Game|GetPlayerCharacter 0)))
  (if (== (Variables|/Game/ThirdPerson/Blueprints/BP_Khris_LightMechanic.BP_Khris_LightMechanic_C|GetLightCollision _asbp_khris_light_mechanic) OtherComp)
    (if (Rendering|IsVisible (Variables|/Game/ThirdPerson/Blueprints/BP_Khris_LightMechanic.BP_Khris_LightMechanic_C|GetLaserLight _asbp_khris_light_mechanic))
      (Utilities|FlowControl|DoOnce false
        (:Completed
          (Game|SpawnActorfromClass "/Game/llave/llave1.llave1_C" (Transformation|GetWorldTransform (Variables|Default|GetKeySpawnPoint)) "AlwaysSpawn" "MultiplyWithRoot" 0 0))))))

(event OnComponentEndOverlap(Box_collision)
  (params (OverlappedComponent :type Primitive%20Component%20Object%20Reference) (OtherActor :type Actor%20Object%20Reference) (OtherComp :type Primitive%20Component%20Object%20Reference) (OtherBodyIndex :type Integer))
  (bind _asbp_khris_light_mechanic (Utilities|Casting|CastToBP_Khris_LightMechanic (Game|GetPlayerCharacter 0)))
  (if (!= (Variables|/Game/ThirdPerson/Blueprints/BP_Khris_LightMechanic.BP_Khris_LightMechanic_C|GetLightCollision _asbp_khris_light_mechanic) 0)
    _))

(event EventBeginPlay)

(event Collision|EventActorBeginOverlap
  (params (OtherActor :type Actor%20Object%20Reference)))

(event EventTick
  (params (DeltaSeconds :type Float%20%28single-precision%29)))

(fn ConstructionScript)