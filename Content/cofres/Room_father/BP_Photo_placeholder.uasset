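; Inspectable photo prop that the player can pick up visually and rotate with the mouse.
; Two trigger volumes, filtering out the player's light collision, drive the camera-facing arrow and icon prompts, with the inner box also toggling input and the Interact widget.
; Interact locks movement and look, then a timeline lerps the photo to BP_Khris_LightMechanic's inspection point.
; Q reverses the timeline, restores control and deactivates the inspection camera.
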(event OnComponentEndOverlap(Box_collision)
  (params (OverlappedComponent :type Primitive%20Component%20Object%20Reference) (OtherActor :type Actor%20Object%20Reference) (OtherComp :type Primitive%20Component%20Object%20Reference) (OtherBodyIndex :type Integer))
  ;[0.15 0.15 0.15 0.5] Interaction
  (Utilities|FlowControl|Sequence
    (:then_0
      ;[0.15 0.15 0.15 0.5] Widget
      (bind _asbp_khris_light_mechanic (Utilities|Casting|CastToBP_Khris_LightMechanic OtherActor))
      (if (!= (Variables|/Game/ThirdPerson/Blueprints/BP_Khris_LightMechanic.BP_Khris_LightMechanic_C|GetLightCollision _asbp_khris_light_mechanic) 0)
        (Input|DisableInput (Game|GetPlayerController 0))
        (Utilities|IsValid (stale OnComponentBeginOverlap(Box_collision) _returnvalue)
          (:Is%20Valid
            (Widget|RemovefromParent (stale OnComponentBeginOverlap(Box_collision) _returnvalue))))))
    (:then_1
      (bind _asbp_khris_light_mechanic_2 (Utilities|Casting|CastToBP_Khris_LightMechanic OtherActor))
      (if (!= (Variables|/Game/ThirdPerson/Blueprints/BP_Khris_LightMechanic.BP_Khris_LightMechanic_C|GetLightCollision _asbp_khris_light_mechanic_2) OtherComp)
        (Development|SetHiddeninGame (Variables|Default|Getinteract_icons) true false)
        (Development|SetHiddeninGame (Variables|Default|Getinteract_arrow) false false)))))

(event OnComponentBeginOverlap(Box_collision)
  (params (OverlappedComponent :type Primitive%20Component%20Object%20Reference) (OtherActor :type Actor%20Object%20Reference) (OtherComp :type Primitive%20Component%20Object%20Reference) (OtherBodyIndex :type Integer) (bFromSweep :type Boolean) (SweepResult :type Hit%20Result%20Structure%20%28by%20ref%29))
  ;[0.15 0.15 0.15 0.5] Interaction
  (Utilities|FlowControl|Sequence
    (:then_0
      ;[0.15 0.15 0.15 0.5] Widget
      (bind _asbp_khris_light_mechanic (Utilities|Casting|CastToBP_Khris_LightMechanic OtherActor))
      (if (!= (Variables|/Game/ThirdPerson/Blueprints/BP_Khris_LightMechanic.BP_Khris_LightMechanic_C|GetLightCollision _asbp_khris_light_mechanic) 0)
        (Input|EnableInput (Game|GetPlayerController 0))
        (bind _returnvalue (UserInterface|CreateWidget "/Game/ui_ux/main_menu/interact.interact_C"))
        (UserInterface|Viewport|AddtoViewport _returnvalue 0)))
    (:then_1
      (bind _asbp_khris_light_mechanic_2 (Utilities|Casting|CastToBP_Khris_LightMechanic OtherActor))
      (if (!= (Variables|/Game/ThirdPerson/Blueprints/BP_Khris_LightMechanic.BP_Khris_LightMechanic_C|GetLightCollision _asbp_khris_light_mechanic_2) OtherComp)
        (Development|SetHiddeninGame (Variables|Default|Getinteract_icons) false false)
        (Development|SetHiddeninGame (Variables|Default|Getinteract_arrow) true false)))))

(event OnComponentBeginOverlap(radius_interact2)
  (params (OverlappedComponent :type Primitive%20Component%20Object%20Reference) (OtherActor :type Actor%20Object%20Reference) (OtherComp :type Primitive%20Component%20Object%20Reference) (OtherBodyIndex :type Integer) (bFromSweep :type Boolean) (SweepResult :type Hit%20Result%20Structure%20%28by%20ref%29))
  ;[0.15 0.15 0.15 0.5] Interaction
  (bind _asbp_khris_light_mechanic (Utilities|Casting|CastToBP_Khris_LightMechanic OtherActor))
  (if (!= (Variables|/Game/ThirdPerson/Blueprints/BP_Khris_LightMechanic.BP_Khris_LightMechanic_C|GetLightCollision _asbp_khris_light_mechanic) OtherComp)
    (Development|SetHiddeninGame (Variables|Default|Getinteract_arrow) false false)))

(event OnComponentEndOverlap(radius_interact2)
  (params (OverlappedComponent :type Primitive%20Component%20Object%20Reference) (OtherActor :type Actor%20Object%20Reference) (OtherComp :type Primitive%20Component%20Object%20Reference) (OtherBodyIndex :type Integer))
  ;[0.15 0.15 0.15 0.5] Interaction
  (bind _asbp_khris_light_mechanic (Utilities|Casting|CastToBP_Khris_LightMechanic OtherActor))
  (if (!= (Variables|/Game/ThirdPerson/Blueprints/BP_Khris_LightMechanic.BP_Khris_LightMechanic_C|GetLightCollision _asbp_khris_light_mechanic) OtherComp)
    (Development|SetHiddeninGame (Variables|Default|Getinteract_arrow) true false)))

(event EventTick
  (params (DeltaSeconds :type Float%20%28single-precision%29))
  ;[0.15 0.15 0.15 0.5] UI Interact always look front
  (Transformation|SetWorldRotation (Variables|Default|Getinteract_icons) (Math|Rotator|MakeRotator 0.0 0.0 (.Yaw (Math|Rotator|BreakRotator (Math|Rotator|CombineRotators (Math|Rotator|FindLookatRotation (Transformation|GetWorldLocation (Variables|Default|Getinteract_icons)) (Camera|GetCameraLocation (Game|GetPlayerCameraManager 0))) "0.000000,-90.000000,0.000000")))) false false))

(event EventBeginPlay
  (bind _photo_placeholder (Variables|Default|GetPhoto_placeholder))
  ;[0.15 0.15 0.15 0.5] get original object position
  (bind _output_get (Variables|Default|SetOriginal%20location (Transformation|GetWorldLocation _photo_placeholder)))
  (bind _output_get_2 (Variables|Default|SetOriginal%20rotation (Transformation|GetWorldRotation _photo_placeholder)))
  (Input|EnableInput (Game|GetPlayerController 0)))

(event EventInteract
  (Development|SetHiddeninGame (Variables|Default|Getinteract_icons) true false)
  (Development|SetHiddeninGame (Variables|Default|Getinteract_arrow) true false)
  (Utilities|IsValid (stale OnComponentBeginOverlap(Box_collision) _returnvalue)
    (:Is%20Valid
      (Widget|RemovefromParent (stale OnComponentBeginOverlap(Box_collision) _returnvalue))
      (Utilities|FlowControl|DoOnce (Variables|Default|GetCan%20inspect?)
        (:Completed
          (Variables|/Script/Engine.PlayerController|SetbShowMouseCursor (Game|GetPlayerController 0) true)
          (Variables|Default|SetCan%20inspect? true)
          (bind _asbp_khris_light_mechanic (Utilities|Casting|CastToBP_Khris_LightMechanic (Game|GetPlayerCharacter 0)))
          (Pawn|Components|CharacterMovement|DisableMovement (Variables|/Script/Engine.Character|GetCharacterMovement (Game|GetPlayerCharacter 0)))
          (Input|SetIgnoreLookInput (Game|GetPlayerController 0) true)
          (bind _newtrack_0 (Timeline|Timeline PlayFromStart)
            (:Update
              (Utilities|IsValid _asbp_khris_light_mechanic
                (:Is%20Valid
                  (Transformation|SetWorldTransform (Variables|Default|GetPhoto_placeholder) (Math|Transform|MakeTransform (Math|Vector|Lerp(Vector) (stale EventBeginPlay _output_get) (.location (Transformation|GetWorldTransform (Variables|/Game/ThirdPerson/Blueprints/BP_Khris_LightMechanic.BP_Khris_LightMechanic_C|GetItemInspectionRef _asbp_khris_light_mechanic))) _newtrack_0) (Math|Rotator|Lerp(Rotator) (stale EventBeginPlay _output_get_2) (.rotation (Transformation|GetWorldTransform (Variables|/Game/ThirdPerson/Blueprints/BP_Khris_LightMechanic.BP_Khris_LightMechanic_C|GetItemInspectionRef _asbp_khris_light_mechanic))) _newtrack_0) "1.000000,1.000000,1.000000") false false))))))))))

(event Input|MouseEvents|MouseX
  (params (AxisValue :type Float%20%28single-precision%29))
  ;[0.15 0.15 0.15 0.5] Rotate object
  (if (Variables|Default|GetCan%20inspect?)
    (Transformation|AddLocalRotation (Variables|Default|GetPhoto_placeholder) (Math|Rotator|MakeRotator 0.0 0.0 (* AxisValue 2.0)) false false)))

(event Input|MouseEvents|MouseY
  (params (AxisValue :type Float%20%28single-precision%29))
  ;[0.15 0.15 0.15 0.5] Rotate object
  (if (Variables|Default|GetCan%20inspect?)
    (Transformation|AddLocalRotation (Variables|Default|GetPhoto_placeholder) (Math|Rotator|MakeRotator 0.0 (* AxisValue -2.0) 0.0) false false)))

(event Input|KeyboardEvents|Q
  (params (Key :type Key%20Structure :default "None"))
  (bind _returnvalue (Game|GetPlayerController 0))
  ;[0.15 0.15 0.15 0.5] Revert inspect
  (:Pressed
    (Development|SetHiddeninGame (Variables|Default|Getinteract_icons) false false)
    (Development|SetHiddeninGame (Variables|Default|Getinteract_arrow) true false)
    (Utilities|FlowControl|Sequence
      (:then_0
        (Utilities|FlowControl|DoOnce (Variables|Default|GetCan%20inspect?)) ; enters at Reset
      )
      (:then_1
        (Variables|Default|SetCan%20inspect? false)
        (Pawn|Components|CharacterMovement|SetMovementMode (Variables|/Script/Engine.Character|GetCharacterMovement (Game|GetPlayerCharacter 0)) "MOVE_Walking" 0)
        (Variables|/Script/Engine.PlayerController|SetbShowMouseCursor _returnvalue false)
        (Input|ResetIgnoreLookInput _returnvalue)
        (Input|SetInputModeGameOnly _returnvalue false)
        (Utilities|FlowControl|Sequence
          (:then_0
            (bind _newtrack_0 (Timeline|Timeline Reverse)
              (:Update
                (Utilities|IsValid (stale EventInteract _asbp_khris_light_mechanic)
                  (:Is%20Valid
                    (Transformation|SetWorldTransform (Variables|Default|GetPhoto_placeholder) (Math|Transform|MakeTransform (Math|Vector|Lerp(Vector) (stale EventBeginPlay _output_get) (.location (Transformation|GetWorldTransform (Variables|/Game/ThirdPerson/Blueprints/BP_Khris_LightMechanic.BP_Khris_LightMechanic_C|GetItemInspectionRef (stale EventInteract _asbp_khris_light_mechanic)))) _newtrack_0) (Math|Rotator|Lerp(Rotator) (stale EventBeginPlay _output_get_2) (.rotation (Transformation|GetWorldTransform (Variables|/Game/ThirdPerson/Blueprints/BP_Khris_LightMechanic.BP_Khris_LightMechanic_C|GetItemInspectionRef (stale EventInteract _asbp_khris_light_mechanic)))) _newtrack_0) "1.000000,1.000000,1.000000") false false))))))
          (:then_1
            (bind _asbp_khris_light_mechanic (Utilities|Casting|CastToBP_Khris_LightMechanic (Game|GetPlayerCharacter 0)))
            (Variables|/Game/ThirdPerson/Blueprints/BP_Khris_LightMechanic.BP_Khris_LightMechanic_C|SetIsIspecting _asbp_khris_light_mechanic false)
            (Default|DeactivateCameraInspection _asbp_khris_light_mechanic)))))))

(fn ConstructionScript)