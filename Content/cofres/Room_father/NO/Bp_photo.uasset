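; Inspectable photo actor that the player can bring up to view and rotate with the mouse.
; Interaction disables movement, shows the cursor and plays a timeline moving the photo to the Khris character's ItemInspectionRef, gated by a DoOnce.
; Both mouse axes feed one local rotation on roll and pitch.
; Q restores movement and game-only input, resets the gate and reverses the timeline to return the photo.
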(event Custom|inspect%20item
  (bind _returnvalue (Transformation|GetActorTransform))
  (bind _as_bp_khris_light_mechanic (Variables|Default|GetAs%20BP%20Khris%20Light%20Mechanic))
  (bind _iteminspectionref (Variables|/Game/ThirdPerson/Blueprints/BP_Khris_LightMechanic.BP_Khris_LightMechanic_C|GetItemInspectionRef _as_bp_khris_light_mechanic))
  (bind _returnvalue_2 (Transformation|GetWorldTransform _iteminspectionref))
  (Utilities|FlowControl|DoOnce false
    (:Completed
      (bind _alpha (Timeline|Rotation_photo Play)
        (:Update
          (Transformation|SetWorldTransform (Variables|Default|Getphoto) (Math|Transform|MakeTransform (Math|Vector|Lerp(Vector) (.location _returnvalue) (.location _returnvalue_2) _alpha) (Math|Rotator|Lerp(Rotator) (.rotation _returnvalue) (.rotation _returnvalue_2) 0.0) "1.000000,1.000000,1.000000") false false))))))

(event Custom|revert
  (bind _returnvalue (Transformation|GetActorTransform))
  (bind _as_bp_khris_light_mechanic (Variables|Default|GetAs%20BP%20Khris%20Light%20Mechanic))
  (bind _iteminspectionref (Variables|/Game/ThirdPerson/Blueprints/BP_Khris_LightMechanic.BP_Khris_LightMechanic_C|GetItemInspectionRef _as_bp_khris_light_mechanic))
  (bind _returnvalue_2 (Transformation|GetWorldTransform _iteminspectionref))
  (Utilities|FlowControl|Sequence
    (:then_0
      (Utilities|FlowControl|DoOnce false) ; enters at Reset
    )
    (:then_1
      (bind _alpha (Timeline|Rotation_photo Reverse)
        (:Update
          (Transformation|SetWorldTransform (Variables|Default|Getphoto) (Math|Transform|MakeTransform (Math|Vector|Lerp(Vector) (.location _returnvalue) (.location _returnvalue_2) _alpha) (Math|Rotator|Lerp(Rotator) (.rotation _returnvalue) (.rotation _returnvalue_2) 0.0) "1.000000,1.000000,1.000000") false false))))))

(event Custom|E_Interaction_1
  (bind _returnvalue (Game|GetPlayerController 0))
  (Pawn|Components|CharacterMovement|DisableMovement (Variables|/Script/Engine.Character|GetCharacterMovement (Game|GetPlayerCharacter 0)))
  (Input|SetIgnoreLookInput _returnvalue false)
  (Input|EnableInput _returnvalue)
  (Variables|/Script/Engine.PlayerController|SetbEnableClickEvents _returnvalue true)
  (Variables|/Script/Engine.PlayerController|SetbShowMouseCursor _returnvalue true)
  (Variables|/Script/Engine.PlayerController|SetbShowMouseCursor _returnvalue true)
  (Input|SetInputModeGameandUI _returnvalue 0 "DoNotLock" true false)
  (CallFunction|InspectItem))

(event EventBeginPlay
  (bind _asbp_khris_light_mechanic (Utilities|Casting|CastToBP_Khris_LightMechanic (Game|GetPlayerCharacter 0)))
  (Variables|Default|SetAs%20BP%20Khris%20Light%20Mechanic _asbp_khris_light_mechanic))

(event Collision|EventActorBeginOverlap
  (params (OtherActor :type Actor%20Object%20Reference)))

(event EventTick
  (params (DeltaSeconds :type Float%20%28single-precision%29)))

(event Input|MouseEvents|MouseX
  (params (AxisValue :type Float%20%28single-precision%29))
  (Transformation|AddLocalRotation (Variables|Default|Getphoto) (Math|Rotator|MakeRotator (* AxisValue 0.4) (* (stale Input|MouseEvents|MouseY AxisValue) 0.4) 0.0) false false))

(event Input|MouseEvents|MouseY
  (params (AxisValue :type Float%20%28single-precision%29))
  (Transformation|AddLocalRotation (Variables|Default|Getphoto) (Math|Rotator|MakeRotator (* (stale Input|MouseEvents|MouseX AxisValue) 0.4) (* AxisValue 0.4) 0.0) false false))

(event Input|KeyboardEvents|Q
  (params (Key :type Key%20Structure :default "None"))
  (bind _returnvalue (Game|GetPlayerController 0))
  (:Pressed
    (Pawn|Components|CharacterMovement|SetMovementMode (Variables|/Script/Engine.Character|GetCharacterMovement (Game|GetPlayerCharacter 0)) "MOVE_Walking" 0)
    (Input|ResetIgnoreLookInput _returnvalue)
    (Input|DisableInput _returnvalue)
    (Variables|/Script/Engine.PlayerController|SetbEnableClickEvents _returnvalue false)
    (Variables|/Script/Engine.PlayerController|SetbShowMouseCursor _returnvalue false)
    (Input|SetInputModeGameOnly _returnvalue false)
    (CallFunction|Revert)))

(fn ConstructionScript)