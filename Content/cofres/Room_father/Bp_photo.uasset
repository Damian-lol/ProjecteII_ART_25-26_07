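; Inspectable photo actor that flies up to the player character's item inspection point.
; On BeginPlay it caches the BP_Khris_LightMechanic player; inspectitem then runs a one-shot timeline moving the Photo mesh toward ItemInspectionRef.
; Only location follows the timeline, as the rotation lerp has no alpha wired.
; A separate NewFunction event, not called here, disables movement and enables cursor, clicks and Game-and-UI input.
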(event Custom|inspect%20item
  (bind _returnvalue (Transformation|GetActorTransform))
  (bind _as_bp_khris_light_mechanic (Variables|Default|GetAs%20BP%20Khris%20Light%20Mechanic))
  (bind _iteminspectionref (Variables|/Game/ThirdPerson/Blueprints/BP_Khris_LightMechanic.BP_Khris_LightMechanic_C|GetItemInspectionRef _as_bp_khris_light_mechanic))
  (bind _returnvalue_2 (Transformation|GetWorldTransform _iteminspectionref))
  (Utilities|FlowControl|DoOnce false
    (:Completed
      (bind _t (Timeline|Rotation_photo Play)
        (:Update
          (Transformation|SetWorldTransform (Variables|Default|Getphoto) (Math|Transform|MakeTransform (Math|Vector|Lerp(Vector) (.location _returnvalue) (.location _returnvalue_2) _t) (Math|Rotator|Lerp(Rotator) (.rotation _returnvalue) (.rotation _returnvalue_2) 0.0) "1.000000,1.000000,1.000000") false false))))))

(event EventBeginPlay
  (bind _asbp_khris_light_mechanic (Utilities|Casting|CastToBP_Khris_LightMechanic (Game|GetPlayerCharacter 0)))
  (Variables|Default|SetAs%20BP%20Khris%20Light%20Mechanic _asbp_khris_light_mechanic))

(event Collision|EventActorBeginOverlap
  (params (OtherActor :type Actor%20Object%20Reference)))

(event EventTick
  (params (DeltaSeconds :type Float%20%28single-precision%29)))

(event EventNewFunction
  (bind _returnvalue (Game|GetPlayerController))
  (Pawn|Components|CharacterMovement|DisableMovement (Variables|/Script/Engine.Character|GetCharacterMovement (Game|GetPlayerCharacter 0)))
  (Input|SetIgnoreLookInput _returnvalue false)
  (Input|EnableInput _returnvalue)
  (Variables|/Script/Engine.PlayerController|SetbEnableClickEvents _returnvalue true)
  (Variables|/Script/Engine.PlayerController|SetbShowMouseCursor _returnvalue true)
  (Variables|/Script/Engine.PlayerController|SetbShowMouseCursor _returnvalue true)
  (Input|SetInputModeGameandUI _returnvalue 0 "DoNotLock" true false))

(fn ConstructionScript)