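; BP_Mirror is a pushable light-puzzle mirror that lights up when illuminated and passes light on to Khris.
; Its box overlap shows an interact widget and enables input, letting E push it along local X through a timeline.
; Sphere overlaps with BP_LightTrigger_2 set Illuminated and drive Activate/Deactivate, fading CylinderLight by timeline.
; A separate collision starts Khris's illumination while the mirror is lit and stops it on exit.
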(event OnComponentBeginOverlap(Collision_for_Krhis)
  (params (OverlappedComponent :type Primitive%20Component%20Object%20Reference) (OtherActor :type Actor%20Object%20Reference) (OtherComp :type Primitive%20Component%20Object%20Reference) (OtherBodyIndex :type Integer) (bFromSweep :type Boolean) (SweepResult :type Hit%20Result%20Structure%20%28by%20ref%29))
  ;[0.15 0.15 0.15 0.5] Khris Light turns on
  (bind _asbp_khris_light_mechanic (Utilities|Casting|CastToBP_Khris_LightMechanic (Game|GetPlayerCharacter 0)))
  (if (!= (Variables|/Game/ThirdPerson/Blueprints/BP_Khris_LightMechanic.BP_Khris_LightMechanic_C|GetLightCollision _asbp_khris_light_mechanic) OtherComp)
    (if (Variables|Default|GetIlluminated)
      (if (Variables|Default|GetActivated)
        (Default|StartIlluminate _asbp_khris_light_mechanic)))))

(event OnComponentEndOverlap(Box)
  (params (OverlappedComponent :type Primitive%20Component%20Object%20Reference) (OtherActor :type Actor%20Object%20Reference) (OtherComp :type Primitive%20Component%20Object%20Reference) (OtherBodyIndex :type Integer))
  ;[0.15 0.15 0.15 0.5] Press E UI
  (bind _asbp_khris_light_mechanic (Utilities|Casting|CastToBP_Khris_LightMechanic (Game|GetPlayerCharacter 0)))
  (if (!= (Variables|/Game/ThirdPerson/Blueprints/BP_Khris_LightMechanic.BP_Khris_LightMechanic_C|GetLightCollision _asbp_khris_light_mechanic) OtherComp)
    (Input|DisableInput (Game|GetPlayerController 0))
    (Widget|RemovefromParent (stale OnComponentBeginOverlap(Box) _returnvalue))))

(event OnComponentEndOverlap(Collision_for_Krhis)
  (params (OverlappedComponent :type Primitive%20Component%20Object%20Reference) (OtherActor :type Actor%20Object%20Reference) (OtherComp :type Primitive%20Component%20Object%20Reference) (OtherBodyIndex :type Integer))
  ;[0.15 0.15 0.15 0.5] Khris Light turns on
  (bind _asbp_khris_light_mechanic (Utilities|Casting|CastToBP_Khris_LightMechanic (Game|GetPlayerCharacter 0)))
  (if (!= (Variables|/Game/ThirdPerson/Blueprints/BP_Khris_LightMechanic.BP_Khris_LightMechanic_C|GetLightCollision _asbp_khris_light_mechanic) OtherComp)
    (Default|StopIlluminate _asbp_khris_light_mechanic)))

(event OnComponentEndOverlap(SphereCollision)
  (params (OverlappedComponent :type Primitive%20Component%20Object%20Reference) (OtherActor :type Actor%20Object%20Reference) (OtherComp :type Primitive%20Component%20Object%20Reference) (OtherBodyIndex :type Integer))
  ;[0.15 0.15 0.15 0.5] Controle whether the player is illuminating this object or not
  (Utilities|Casting|CastToBP_LightTrigger_2 OtherActor)
  (if true
    (Variables|Default|SetIlluminated false)
    (Development|PrintString "--- NOT ILLUMINATED")
    ;[0.15 0.15 0.15 0.5] Controls whether the object should acticate or not
    (if (Variables|Default|GetIlluminated)
      (if (Variables|Default|GetActivated)
        (CallFunction|Deactivate)
        (else
          (CallFunction|Activate)))
      (elif (Variables|Default|GetActivated)
        (CallFunction|Deactivate)))))

(event OnComponentBeginOverlap(SphereCollision)
  (params (OverlappedComponent :type Primitive%20Component%20Object%20Reference) (OtherActor :type Actor%20Object%20Reference) (OtherComp :type Primitive%20Component%20Object%20Reference) (OtherBodyIndex :type Integer) (bFromSweep :type Boolean) (SweepResult :type Hit%20Result%20Structure%20%28by%20ref%29))
  ;[0.15 0.15 0.15 0.5] Controle whether the player is illuminating this object or not
  (Utilities|Casting|CastToBP_LightTrigger_2 OtherActor)
  (Variables|Default|SetIlluminated true)
  (Development|PrintString "--- ILLUMINATED")
  ;[0.15 0.15 0.15 0.5] Controls whether the object should acticate or not
  (if (Variables|Default|GetIlluminated)
    (if (Variables|Default|GetActivated)
      (CallFunction|Deactivate)
      (else
        (CallFunction|Activate)))
    (elif (Variables|Default|GetActivated)
      (CallFunction|Deactivate))))

(event OnComponentBeginOverlap(Box)
  (params (OverlappedComponent :type Primitive%20Component%20Object%20Reference) (OtherActor :type Actor%20Object%20Reference) (OtherComp :type Primitive%20Component%20Object%20Reference) (OtherBodyIndex :type Integer) (bFromSweep :type Boolean) (SweepResult :type Hit%20Result%20Structure%20%28by%20ref%29))
  ;[0.15 0.15 0.15 0.5] Press E UI
  (bind _asbp_khris_light_mechanic (Utilities|Casting|CastToBP_Khris_LightMechanic (Game|GetPlayerCharacter 0)))
  (if (!= (Variables|/Game/ThirdPerson/Blueprints/BP_Khris_LightMechanic.BP_Khris_LightMechanic_C|GetLightCollision _asbp_khris_light_mechanic) OtherComp)
    (Input|EnableInput (Game|GetPlayerController 0))
    (bind _returnvalue (UserInterface|CreateWidget "/Game/ui_ux/main_menu/interact.interact_C"))
    (UserInterface|Viewport|AddtoViewport _returnvalue 0)))

(event Custom|Activate
  ;[0.15 0.15 0.15 0.5] Light contorls (brighten and dim)
  (Variables|Default|SetActivated true)
  (Development|PrintString "--- ACTIVATED")
  (bind _intensity (Timeline|Timeline Play)
    (:Update
      (Rendering|Components|Light|SetIntensity (Variables|Default|GetCylinderLight) (Math|Float|Lerp 0.0 5e+03 _intensity)))))

(event Custom|Deactivate
  ;[0.15 0.15 0.15 0.5] Light contorls (brighten and dim)
  (Variables|Default|SetActivated false)
  (Development|PrintString "--- DEACTIVATED")
  (bind _intensity (Timeline|Timeline Reverse)
    (:Update
      (Rendering|Components|Light|SetIntensity (Variables|Default|GetCylinderLight) (Math|Float|Lerp 0.0 5e+03 _intensity)))))

(event Input|KeyboardEvents|E
  (params (Key :type Key%20Structure :default "None"))
  ;[0.15 0.15 0.15 0.5] Press E to push object
  (:Pressed
    (Utilities|Casting|CastToBP_Khris_LightMechanic (Game|GetPlayerCharacter 0))
    (bind _movimiento (Timeline|Timeline_0 Play)
      (:Update
        (Transformation|AddActorLocalOffset (Math|Vector|MakeVector (Math|Float|Lerp (Variables|Default|GetA) (Variables|Default|GetB) _movimiento) 0.0 0.0) false false)
        (Utilities|FlowControl|DoOnce false)))))

(fn ConstructionScript)

(fn IsPlayerIlluminated
  (bind _asbp_khris_light_mechanic (Utilities|Casting|CastToBP_Khris_LightMechanic (Game|GetPlayerCharacter 0))
    (:then
      (return (Variables|/Game/ThirdPerson/Blueprints/BP_Khris_LightMechanic.BP_Khris_LightMechanic_C|GetEstaIluminada _asbp_khris_light_mechanic)))
    (:CastFailed
      (return false))))