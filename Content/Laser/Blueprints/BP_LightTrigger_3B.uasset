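; BP_LightTrigger_3B is a light trigger volume that reacts to BP_Khris_LightMechanic entering its sphere, depending on whether the BP_Mirror is placed.
; Without a placed mirror, it starts illumination and fades in a light sound.
; With one, it clears the lit flag, briefly disables input while a timeline nudges the player backward, and stops illumination.
; Leaving the sphere shares that stop branch, which also fades out the sound.
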(event OnComponentBeginOverlap(Sphere)
  (params (OverlappedComponent :type Primitive%20Component%20Object%20Reference) (OtherActor :type Actor%20Object%20Reference) (OtherComp :type Primitive%20Component%20Object%20Reference) (OtherBodyIndex :type Integer) (bFromSweep :type Boolean) (SweepResult :type Hit%20Result%20Structure%20%28by%20ref%29))
  (bind _returnvalue (Game|GetPlayerCharacter 0))
  (bind _asbp_khris_light_mechanic (Utilities|Casting|CastToBP_Khris_LightMechanic OtherActor))
  (if (!= (Variables|/Game/ThirdPerson/Blueprints/BP_Khris_LightMechanic.BP_Khris_LightMechanic_C|GetLightCollision _asbp_khris_light_mechanic) OtherComp)
    (bind _returnvalue_2 (Actor|GetActorOfClass "/Game/reflective_objects/BP_Mirror.BP_Mirror_C"))
    (Utilities|IsValid _returnvalue_2
      (:Is%20Valid
        (if (Variables|/Game/reflective_objects/BP_Mirror.BP_Mirror_C|GetIsMirrorPlaced? _returnvalue_2)
          (Variables|/Game/ThirdPerson/Blueprints/BP_Khris_LightMechanic.BP_Khris_LightMechanic_C|SetEstaIluminada _asbp_khris_light_mechanic false)
          (Utilities|FlowControl|Sequence
            (:then_0
              (Input|DisableInput (Game|GetPlayerCharacter 0) (Game|GetPlayerController 0))
              (Variables|Default|SetStartPosition (Transformation|GetActorLocation _returnvalue))
              (Variables|Default|SetEndPosition (+ (Variables|Default|GetStartPosition) (* (Transformation|GetActorForwardVector _returnvalue) -2e+01)))
              (bind _newtrack_0 (Timeline|Timeline PlayFromStart)
                (:Update
                  (Transformation|SetActorLocation (Game|GetPlayerCharacter 0) (Math|Vector|Lerp(Vector) (Variables|Default|GetStartPosition) (Variables|Default|GetEndPosition) _newtrack_0) false false))
                (:Finished
                  (Input|EnableInput (Game|GetPlayerCharacter 0) (Game|GetPlayerController 0)))))
            (:then_1
              (Default|StopIlluminate (stale OnComponentEndOverlap(Sphere) _asbp_khris_light_mechanic))
              (Utilities|IsValid (stale _returnvalue_3)
                (:Is%20Valid
                  (Audio|Components|Audio|FadeOut (stale _returnvalue_3) 0.5 0.0 "Sin" :!class /Script/Engine.AudioComponent)))))
          (else
            (Default|StartIlluminate _asbp_khris_light_mechanic)
            (bind _returnvalue_3 (Audio|SpawnSound2D "/Game/Audio/SoundDesign/03_SFX/Luz/SC_Luz.SC_Luz" 1.0 1.0 0.0 0))
            (Audio|Components|Audio|FadeIn _returnvalue_3 2.0 1.0 0.0 "Sin" :!class /Script/Engine.AudioComponent)))))))

(event OnComponentEndOverlap(Sphere)
  (params (OverlappedComponent :type Primitive%20Component%20Object%20Reference) (OtherActor :type Actor%20Object%20Reference) (OtherComp :type Primitive%20Component%20Object%20Reference) (OtherBodyIndex :type Integer))
  (bind _asbp_khris_light_mechanic (Utilities|Casting|CastToBP_Khris_LightMechanic OtherActor))
  (if (!= (Variables|/Game/ThirdPerson/Blueprints/BP_Khris_LightMechanic.BP_Khris_LightMechanic_C|GetLightCollision _asbp_khris_light_mechanic) OtherComp)
    (Utilities|IsValid _asbp_khris_light_mechanic
      (:Is%20Valid
        (Default|StopIlluminate _asbp_khris_light_mechanic)
        (Utilities|IsValid (stale OnComponentBeginOverlap(Sphere) _returnvalue_3)
          (:Is%20Valid
            (Audio|Components|Audio|FadeOut (stale OnComponentBeginOverlap(Sphere) _returnvalue_3) 0.5 0.0 "Sin" :!class /Script/Engine.AudioComponent)))))))

(event EventTick
  (params (DeltaSeconds :type Float%20%28single-precision%29)))

(fn ConstructionScript)

(fn IluminationActualización)