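; BP_Music_Manager switches FMOD music as the game moves between house areas such as Khris's room, the upstairs hallway, dining room and living room.
; Area events fade out playing audio through a bus stop, then start their 2D track; Khris's room does this only once.
; Trigger events set parameters on the saved hallway and dining-room instances to vary the music for melodies and the father's room.
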(event Custom|Hab%20Pare
  (Class|FMODBlueprintStatics|EventInstanceSetParameter (stale Custom|Lv1%20enter _returnvalue) "Hab_pare_s_n" 1.0))

(event Custom|Lv1%20enter
  (Class|FMODBlueprintStatics|BusStopAllEvents "/Game/FMOD/Buses/Stop_bus.Stop_bus" "ALLOWFADEOUT")
  (bind _returnvalue (Class|FMODBlueprintStatics|PlayEvent2D "/Game/FMOD/Events/Passadís_dalt_+_hab_pare.Passadís_dalt_+_hab_pare")))

(event Custom|MelodyTrigger2
  (Class|FMODBlueprintStatics|EventInstanceSetParameter (stale Custom|Menjador%20enter _returnvalue) "Nota" 1.0))

(event Custom|Menjador%20enter
  (Class|FMODBlueprintStatics|BusStopAllEvents "/Game/FMOD/Buses/Stop_bus.Stop_bus" "ALLOWFADEOUT")
  (bind _returnvalue (Class|FMODBlueprintStatics|PlayEvent2D "/Game/FMOD/Events/Menjador.Menjador")))

(event Custom|Melody%20trigger
  (Class|FMODBlueprintStatics|EventInstanceSetParameter (stale Custom|Lv1%20enter _returnvalue) "Foto_s_n" 1.0))

(event Custom|Sala%20enter
  (Class|FMODBlueprintStatics|BusStopAllEvents "/Game/FMOD/Buses/Stop_bus.Stop_bus" "ALLOWFADEOUT")
  (Class|FMODBlueprintStatics|PlayEvent2D "/Game/FMOD/Events/Sala_d_estar.Sala_d_estar"))

(event Custom|Hab%20Khris
  (Utilities|FlowControl|DoOnce false
    (:Completed
      (Class|FMODBlueprintStatics|BusStopAllEvents 0 "ALLOWFADEOUT")
      (Class|FMODBlueprintStatics|PlayEvent2D "/Game/FMOD/Events/Hab_Khris.Hab_Khris"))))