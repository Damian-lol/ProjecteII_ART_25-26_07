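; BP_Trigger_pasillo2 is a trigger volume that shows a hallway dialogue box when Khris walks into it.
; Overlaps from BP_Khris_LightMechanic count only if the overlapping component is not the character's LightCollision.
; A DoOnce gate creates the dialogue widget, plays a warning sound and fades the box in.
; After a short delay it fades out and resets the gate, so the trigger can fire again.
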(event OnComponentBeginOverlap(CollisionComponent)
  (params (OverlappedComponent :type Primitive%20Component%20Object%20Reference) (OtherActor :type Actor%20Object%20Reference) (OtherComp :type Primitive%20Component%20Object%20Reference) (OtherBodyIndex :type Integer) (bFromSweep :type Boolean) (SweepResult :type Hit%20Result%20Structure%20%28by%20ref%29))
  (bind _asbp_khris_light_mechanic (Utilities|Casting|CastToBP_Khris_LightMechanic OtherActor))
  (if (!= (Variables|/Game/ThirdPerson/Blueprints/BP_Khris_LightMechanic.BP_Khris_LightMechanic_C|GetLightCollision _asbp_khris_light_mechanic) OtherComp)
    (Utilities|FlowControl|DoOnce false :!label _label
      (:Completed
        (bind _returnvalue (UserInterface|CreateWidget "/Game/Dialogue/WBP_DialogueBox1Khris_Pasillo.WBP_DialogueBox1Khris_Pasillo_C"))
        (Audio|PlaySound2D "/Game/Audio/SoundDesign/03_SFX/GuidingLight/Aviso/SC_GL_Aviso.SC_GL_Aviso" 1.0 1.0 0.0 0 0)
        (bind _output_get (Variables|Default|SetDialogueReferenceWidget _returnvalue))
        (UserInterface|Viewport|AddtoViewport _output_get 0)
        (Default|FadeinAnim (Variables|Default|GetDialogueReferenceWidget))
        (Utilities|FlowControl|Delay 2.5)
        (Default|FadeOutAnim (Variables|Default|GetDialogueReferenceWidget))
        (goto _label Reset)))))

(event EventBeginPlay)

(event Collision|EventActorBeginOverlap
  (params (OtherActor :type Actor%20Object%20Reference)))

(event EventTick
  (params (DeltaSeconds :type Float%20%28single-precision%29)))

(fn ConstructionScript)