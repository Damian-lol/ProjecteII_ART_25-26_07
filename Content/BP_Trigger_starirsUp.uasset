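; Trigger volume, named for an upward staircase, that reacts when BP_Khris_LightMechanic overlaps it with any component other than its LightCollision.
; The overlap issues a zero-velocity launch on the player and plays the GoBack timeline.
; GoBack moves the trigger actor itself from the player's location to a point far behind the player.
; A DoOnce on the timeline update briefly fades a WBP_DialogueBox in and out, resetting afterward.
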(event OnComponentBeginOverlap(CollisionComponent)
  (params (OverlappedComponent :type Primitive%20Component%20Object%20Reference) (OtherActor :type Actor%20Object%20Reference) (OtherComp :type Primitive%20Component%20Object%20Reference) (OtherBodyIndex :type Integer) (bFromSweep :type Boolean) (SweepResult :type Hit%20Result%20Structure%20%28by%20ref%29))
  (bind _returnvalue (Game|GetPlayerCharacter 0))
  (bind _asbp_khris_light_mechanic (Utilities|Casting|CastToBP_Khris_LightMechanic OtherActor))
  (if (!= (Variables|/Game/ThirdPerson/Blueprints/BP_Khris_LightMechanic.BP_Khris_LightMechanic_C|GetLightCollision _asbp_khris_light_mechanic) OtherComp)
    (Variables|Default|SetStartPosition (Transformation|GetActorLocation _returnvalue))
    (Variables|Default|SetEndPosition (+ (Variables|Default|GetStartPosition) (* (Transformation|GetActorForwardVector _returnvalue) -2e+03)))
    (Character|LaunchCharacter _returnvalue "0, 0, 0" false false)
    (bind _newtrack_0 (Timeline|GoBack PlayFromStart)
      (:Update
        (Transformation|SetActorLocation (Math|Vector|Lerp(Vector) (Variables|Default|GetStartPosition) (Variables|Default|GetEndPosition) _newtrack_0) false false)
        (Utilities|FlowControl|DoOnce false :!label _label
          (:Completed
            (bind _returnvalue_2 (UserInterface|CreateWidget "/Game/Dialogue/WBP_DialogueBox.WBP_DialogueBox_C"))
            (bind _output_get (Variables|Default|SetwIdgetDialogueReference _returnvalue_2))
            (UserInterface|Viewport|AddtoViewport _output_get 0)
            (Default|FadeinAnim (Variables|Default|GetwIdgetDialogueReference))
            (Utilities|FlowControl|Delay 2.0)
            (Default|FadeOutAnim (Variables|Default|GetwIdgetDialogueReference))
            (goto _label Reset)))))))

(event EventBeginPlay)

(event Collision|EventActorBeginOverlap
  (params (OtherActor :type Actor%20Object%20Reference)))

(event EventTick
  (params (DeltaSeconds :type Float%20%28single-precision%29)))

(fn ConstructionScript)