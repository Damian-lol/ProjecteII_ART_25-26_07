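; BP_candado is a padlock actor that dissolves when the player shines the flashlight on it.
; When BP_Khris_LightMechanic's light collision overlaps the box while the flashlight effect is visible, a one-shot swaps the lock's material and makes it dynamic.
; A timeline drives its Dissolve parameter, then the lock component is destroyed and, after a short delay, the actor.
; The end-overlap handler only casts to BP_Mirror, and its sound-stop logic is disconnected.
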(event OnComponentBeginOverlap(Box_collision)
  (params (OverlappedComponent :type Primitive%20Component%20Object%20Reference) (OtherActor :type Actor%20Object%20Reference) (OtherComp :type Primitive%20Component%20Object%20Reference) (OtherBodyIndex :type Integer) (bFromSweep :type Boolean) (SweepResult :type Hit%20Result%20Structure%20%28by%20ref%29))
  (bind _lock (Variables|Default|Getlock))
  ;[0.15 0.15 0.15 0.5] Free door
  (bind _asbp_khris_light_mechanic (Utilities|Casting|CastToBP_Khris_LightMechanic OtherActor))
  (if (and (Rendering|IsVisible (Variables|/Game/ThirdPerson/Blueprints/BP_Khris_LightMechanic.BP_Khris_LightMechanic_C|GetFlashlightFX _asbp_khris_light_mechanic)) (== (Variables|/Game/ThirdPerson/Blueprints/BP_Khris_LightMechanic.BP_Khris_LightMechanic_C|GetLightCollision _asbp_khris_light_mechanic) OtherComp))
    (Utilities|FlowControl|DoOnce false
      (:Completed
        (Rendering|Material|SetMaterial _lock 0 "/Game/Crystal/Crystal_Inst_final_candado.Crystal_Inst_final_candado")
        (bind _returnvalue (Rendering|Material|CreateDynamicMaterialInstance _lock 0 (Rendering|Material|GetMaterial _lock 0) "None" :!class /Script/Engine.PrimitiveComponent))
        (bind _output_get (Variables|Default|SetDissolveMat _returnvalue))
        (bind _dissolveanim (Timeline|DissolveAnim PlayFromStart)
          (:Update
            (Rendering|Material|SetScalarParameterValue _output_get "Dissolve" (Math|Float|Lerp -0.4 0.7 _dissolveanim) :!class /Script/Engine.MaterialInstanceDynamic))
          (:Finished
            (Components|DestroyComponent (Variables|Default|Getlock))
            (Utilities|FlowControl|Delay 1.0)
            (Actor|DestroyActor)))))))

(event OnComponentEndOverlap(Box_collision)
  (params (OverlappedComponent :type Primitive%20Component%20Object%20Reference) (OtherActor :type Actor%20Object%20Reference) (OtherComp :type Primitive%20Component%20Object%20Reference) (OtherBodyIndex :type Integer))
  ;[0.15 0.15 0.15 0.5] Free door
  (Utilities|Casting|CastToBP_Mirror OtherActor))

(event Collision|EventActorBeginOverlap
  (params (OtherActor :type Actor%20Object%20Reference)))

(event EventTick
  (params (DeltaSeconds :type Float%20%28single-precision%29)))

(fn ConstructionScript)