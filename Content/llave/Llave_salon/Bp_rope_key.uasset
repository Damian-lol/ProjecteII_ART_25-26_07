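; Rope holding the living room key, which burns away to free it when hit by the player's flashlight while a mirror is in place.
; A BP_Mirror overlap arms the burn with sound and smoke; a later overlap by Khris's visible flashlight collision starts it.
; A timeline drives a dynamic dissolve material, then flags the rope destroyed on the key, enables key physics, plays sounds and removes rope and smoke.
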(event OnComponentBeginOverlap(Box_collision)
  (params (OverlappedComponent :type Primitive%20Component%20Object%20Reference) (OtherActor :type Actor%20Object%20Reference) (OtherComp :type Primitive%20Component%20Object%20Reference) (OtherBodyIndex :type Integer) (bFromSweep :type Boolean) (SweepResult :type Hit%20Result%20Structure%20%28by%20ref%29))
  (bind _asbp_khris_light_mechanic (Utilities|Casting|CastToBP_Khris_LightMechanic OtherActor))
  (bind _rope (Variables|Default|Getrope))
  (bind _rope_2 (Variables|Default|Getrope))
  (bind _key_livingroom (Variables|Default|GetKey_LivingRoom))
  (bind _returnvalue (Transformation|GetWorldLocation _rope))
  ;[0.15 0.15 0.15 0.5] Free key
  (Utilities|Casting|CastToBP_Mirror OtherActor
    (:then
      (Variables|Default|SetMirrorLightIsTouching? true)
      (bind _returnvalue_2 (Audio|SpawnSoundatLocation "/Game/Audio/SoundDesign/04_Foley/Cuerda/Rompiendose/SC_Cuerda_Rompiendose.SC_Cuerda_Rompiendose" _returnvalue "0, 0, 0" 0.75 1.0 0.0 "/Game/AS_Rope.AS_Rope" 0))
      (Variables|Default|SetBurningRope _returnvalue_2)
      (bind _returnvalue_3 (Effects|SpawnEmitteratLocation "/Game/fx/P_Smoke.P_Smoke" "-23.627064,5277.331243,207.378024" "0, 0, 0" "0.300000,0.300000,0.300000")))
    (:CastFailed
      (Utilities|IsValid _asbp_khris_light_mechanic
        (:Is%20Valid
          (if (Math|Boolean|ANDBoolean (Rendering|IsVisible (Variables|/Game/ThirdPerson/Blueprints/BP_Khris_LightMechanic.BP_Khris_LightMechanic_C|GetFlashlightFX _asbp_khris_light_mechanic)) (== (Variables|/Game/ThirdPerson/Blueprints/BP_Khris_LightMechanic.BP_Khris_LightMechanic_C|GetLightCollision _asbp_khris_light_mechanic) OtherComp) (Variables|Default|GetMirrorLightIsTouching?))
            (Utilities|IsValid _rope_2
              (:Is%20Valid
                (Rendering|Material|SetMaterial _rope_2 0 "/Game/fx/M_Dissolve_Inst.M_Dissolve_Inst")
                (bind _returnvalue_4 (Rendering|Material|CreateDynamicMaterialInstance _rope_2 0 (Rendering|Material|GetMaterial _rope_2 0) "None" :!class /Script/Engine.PrimitiveComponent))
                (bind _output_get (Variables|Default|SetDissolveMat _returnvalue_4))
                (bind _dissolveanim (Timeline|DissolveAnim PlayFromStart)
                  (:Update
                    (Rendering|Material|SetScalarParameterValue _output_get "Dissolve" (Math|Float|Lerp -0.4 0.7 _dissolveanim) :!class /Script/Engine.MaterialInstanceDynamic))
                  (:Finished
                    (Variables|/Game/llave/Llave_salon/llave_salon.llave_salon_C|SetIs%20rope%20destroyed? _key_livingroom true)
                    (Utilities|FlowControl|DoOnce false
                      (:Completed
                        (Physics|SetSimulatePhysics (Variables|/Game/llave/Llave_salon/llave_salon.llave_salon_C|Getllave _key_livingroom) true)
                        (Utilities|FlowControl|Sequence
                          (:then_0
                            (Audio|Components|Audio|Stop _returnvalue_2)
                            (Audio|SpawnSoundatLocation "/Game/Audio/SoundDesign/04_Foley/Cuerda/Rompiendose/SnapCuerda.SnapCuerda" _returnvalue "0, 0, 0" 1.0 1.0 0.0 "/Game/AS_Rope.AS_Rope" 0))
                          (:then_1
                            (Components|DestroyComponent (Variables|Default|Getrope))
                            (Utilities|FlowControl|Delay 0.6)
                            (Audio|PlaySoundatLocation "/Game/Audio/SoundDesign/04_Foley/Llaves_Suelo/SC_Llaves.SC_Llaves" "0, 0, 0" "0, 0, 0" 1.0 1.0 0.0 "/Game/AS_Rope.AS_Rope" 0 0 0)))))))))))))))

(event OnComponentEndOverlap(Box_collision)
  (params (OverlappedComponent :type Primitive%20Component%20Object%20Reference) (OtherActor :type Actor%20Object%20Reference) (OtherComp :type Primitive%20Component%20Object%20Reference) (OtherBodyIndex :type Integer))
  (bind _burningrope (Variables|Default|GetBurningRope))
  ;[0.15 0.15 0.15 0.5] Free key
  (Utilities|Casting|CastToBP_Mirror OtherActor)
  (Variables|Default|SetMirrorLightIsTouching? false)
  (Utilities|IsValid _burningrope
    (:Is%20Valid
      (Audio|Components|Audio|Stop _burningrope))))

(event Collision|EventActorBeginOverlap
  (params (OtherActor :type Actor%20Object%20Reference)))

(event EventTick
  (params (DeltaSeconds :type Float%20%28single-precision%29)))

(fn ConstructionScript)