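; BP_rope_door is a rope blocking the living room door, burned or freed through a mirror and laser light puzzle.
; Its collision box tracks whether a BP_Mirror overlaps it.
; When Khris's light collision then begins overlapping with the laser visible and the mirror present, it sets RopeIsNotLongerBlocking on Puerta_LivingRoom and destroys the rope once.
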(event OnComponentBeginOverlap(Box_collision)
  (params (OverlappedComponent :type Primitive%20Component%20Object%20Reference) (OtherActor :type Actor%20Object%20Reference) (OtherComp :type Primitive%20Component%20Object%20Reference) (OtherBodyIndex :type Integer) (bFromSweep :type Boolean) (SweepResult :type Hit%20Result%20Structure%20%28by%20ref%29))
  (bind _asbp_khris_light_mechanic (Utilities|Casting|CastToBP_Khris_LightMechanic OtherActor))
  ;[0.15 0.15 0.15 0.5] Free door
  (Utilities|Casting|CastToBP_Mirror OtherActor
    (:then
      (Variables|Default|SetMirror%20illuminating? true))
    (:CastFailed
      (Utilities|IsValid _asbp_khris_light_mechanic
        (:Is%20Valid
          (if (Math|Boolean|ANDBoolean (Rendering|IsVisible (Variables|/Game/ThirdPerson/Blueprints/BP_Khris_LightMechanic.BP_Khris_LightMechanic_C|GetLaserLight _asbp_khris_light_mechanic)) (== (Variables|/Game/ThirdPerson/Blueprints/BP_Khris_LightMechanic.BP_Khris_LightMechanic_C|GetLightCollision _asbp_khris_light_mechanic) OtherComp) (Variables|Default|GetMirror%20illuminating?))
            (Utilities|FlowControl|DoOnce false
              (:Completed
                (bind _returnvalue (Actor|GetActorOfClass "/Game/puerta_LivingRoom.puerta_LivingRoom_C"))
                (Variables|/Game/puerta_LivingRoom.puerta_LivingRoom_C|SetRopeIsNotLongerBlocking _returnvalue true)
                (Components|DestroyComponent (Variables|Default|Getrope))))))))))

(event OnComponentEndOverlap(Box_collision)
  (params (OverlappedComponent :type Primitive%20Component%20Object%20Reference) (OtherActor :type Actor%20Object%20Reference) (OtherComp :type Primitive%20Component%20Object%20Reference) (OtherBodyIndex :type Integer))
  ;[0.15 0.15 0.15 0.5] Free door
  (Utilities|Casting|CastToBP_Mirror OtherActor)
  (Variables|Default|SetMirror%20illuminating? false))

(event EventBeginPlay)

(event Collision|EventActorBeginOverlap
  (params (OtherActor :type Actor%20Object%20Reference)))

(event EventTick
  (params (DeltaSeconds :type Float%20%28single-precision%29)))

(fn ConstructionScript)