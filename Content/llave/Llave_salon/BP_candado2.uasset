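; Padlock actor that dissolves and removes itself once it is triggered to free a door.
; The door-open event sets DoolMelt and calls Melt, which proceeds once, only if the Altar_doll's flashlight FX and cylinder light are both visible.
; A timeline then animates the Dissolve parameter on a dynamic crystal material, destroys the lock mesh and, after a short delay, the actor.
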(event OnComponentBeginOverlap(Box_collision)
  (params (OverlappedComponent :type Primitive%20Component%20Object%20Reference) (OtherActor :type Actor%20Object%20Reference) (OtherComp :type Primitive%20Component%20Object%20Reference) (OtherBodyIndex :type Integer) (bFromSweep :type Boolean) (SweepResult :type Hit%20Result%20Structure%20%28by%20ref%29)))

(event Custom|door_open?
  ;[0.15 0.15 0.15 0.5] Free door
  (Variables|Default|Setdool_melt? true)
  (CallFunction|Melt?))

(event Custom|timeline
  (bind _lock (Variables|Default|Getlock))
  ;[0.15 0.15 0.15 0.5] Free door
  (Rendering|Material|SetMaterial _lock 0 "/Game/Crystal/Crystal_Inst_final_candado.Crystal_Inst_final_candado")
  (bind _returnvalue (Rendering|Material|CreateDynamicMaterialInstance _lock 0 (Rendering|Material|GetMaterial _lock 0) "None" :!class /Script/Engine.PrimitiveComponent))
  (bind _output_get (Variables|Default|Setmaterial _returnvalue))
  (bind _dissolveanim (Timeline|Cronograma Play)
    (:Update
      (Rendering|Material|SetScalarParameterValue _output_get "Dissolve" (Math|Float|Lerp -0.4 0.7 _dissolveanim) :!class /Script/Engine.MaterialInstanceDynamic))
    (:Finished
      (Components|DestroyComponent (Variables|Default|Getlock))
      (Utilities|FlowControl|Delay 1.0)
      (Actor|DestroyActor))))

(event Collision|EventActorBeginOverlap
  (params (OtherActor :type Actor%20Object%20Reference)))

(event EventTick
  (params (DeltaSeconds :type Float%20%28single-precision%29)))

(fn ConstructionScript)

(fn Melt?
  (if (Variables|Default|Getdool_melt?)
    (bind _returnvalue (Actor|GetActorOfClass "/Game/doll_pick_up/altar_doll.altar_doll_C"))
    (if (and (Rendering|IsVisible (Variables|/Game/doll_pick_up/altar_doll.altar_doll_C|GetFlashLightFX _returnvalue)) (Rendering|IsVisible (Variables|/Game/doll_pick_up/altar_doll.altar_doll_C|GetCylinderLight _returnvalue)))
      (Utilities|FlowControl|DoOnce false
        (:Completed
          (CallFunction|Timeline))))))

(fn OnRepDoolMelt?)