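; Kitchen cabinet that guards a key (dining-room key, per its folder) and opens when Khris overlaps its box with the laser light visible.
; It disables input, blends to a cabinet camera, plays a sound and swings the door via a Timeline on an Arrow, then restores control.
; When the swing finishes, key pickup is enabled; until then, the interaction sphere shows a brief fading dialogue, ignoring the light's collision.
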(event OnComponentBeginOverlap(SphereInteraction)
  (params (OverlappedComponent :type Primitive%20Component%20Object%20Reference) (OtherActor :type Actor%20Object%20Reference) (OtherComp :type Primitive%20Component%20Object%20Reference) (OtherBodyIndex :type Integer) (bFromSweep :type Boolean) (SweepResult :type Hit%20Result%20Structure%20%28by%20ref%29))
  ;[0.15 0.15 0.15 0.5] It's closed dialogue
  (bind _asbp_khris_light_mechanic (Utilities|Casting|CastToBP_Khris_LightMechanic OtherActor))
  (if (!= (Variables|/Game/ThirdPerson/Blueprints/BP_Khris_LightMechanic.BP_Khris_LightMechanic_C|GetLightCollision _asbp_khris_light_mechanic) OtherComp)
    (if (not (Variables|Default|Getcan%20pick%20key?))
      (Utilities|FlowControl|DoOnce false :!label _label
        (:Completed
          (bind _returnvalue (UserInterface|CreateWidget "/Game/Dialogue/WBP_DialogueBox1Khris.WBP_DialogueBox1Khris_C"))
          (bind _output_get (Variables|Default|SetWidgetDialogueReference _returnvalue))
          (UserInterface|Viewport|AddtoViewport _output_get 0)
          (Default|FadeinAnim (Variables|Default|GetWidgetDialogueReference))
          (Utilities|FlowControl|Delay 2.0)
          (Default|FadeOutAnim (Variables|Default|GetWidgetDialogueReference))
          (goto _label Reset))))))

(event OnComponentBeginOverlap(Box_collision)
  (params (OverlappedComponent :type Primitive%20Component%20Object%20Reference) (OtherActor :type Actor%20Object%20Reference) (OtherComp :type Primitive%20Component%20Object%20Reference) (OtherBodyIndex :type Integer) (bFromSweep :type Boolean) (SweepResult :type Hit%20Result%20Structure%20%28by%20ref%29))
  (bind _asbp_khris_light_mechanic (Utilities|Casting|CastToBP_Khris_LightMechanic OtherActor))
  (if (Rendering|IsVisible (Variables|/Game/ThirdPerson/Blueprints/BP_Khris_LightMechanic.BP_Khris_LightMechanic_C|GetLaserLight _asbp_khris_light_mechanic))
    (if (not (Variables|Default|GetCabinetDoorOpened?))
      (Input|DisableInput (Game|GetPlayerCharacter 0) (Game|GetPlayerController 0))
      (Game|Player|SetViewTargetwithBlend (Game|GetPlayerController 0) (Variables|Default|GetKeySpawnedCamera) 2.0 "VTBlend_Cubic" 0.0 false)
      (Utilities|FlowControl|Delay 1.5)
      ;[0.15 0.15 0.15 0.5] Open cabinet door
      (Utilities|FlowControl|DoOnce false
        (:Completed
          (Audio|PlaySound2D "/Game/Audio/SoundDesign/04_Foley/Armario/PuertaArmarioCocina.PuertaArmarioCocina" 1.0 1.0 0.0 0 0)
          (bind __puerta (Timeline|Timeline Play)
            (:Update
              (Transformation|SetRelativeRotation (Variables|Default|GetArrow) (Math|Rotator|MakeRotator 0.0 0.0 (Math|Float|Lerp (Variables|Default|Getpuerta%20cerrada) (Variables|Default|Getpuerta%20abierta) __puerta)) false false)
              (Utilities|FlowControl|Delay 1.0)
              (Game|Player|SetViewTargetwithBlend (Game|GetPlayerController 0) (Game|GetPlayerCharacter 0) 2.0 "VTBlend_Cubic" 0.0 false)
              (Input|EnableInput (Game|GetPlayerCharacter 0) (Game|GetPlayerController 0))
              (Variables|Default|SetCabinetDoorOpened? true))
            (:Finished
              (Variables|Default|Setcan%20pick%20key? true))))))))

(fn ConstructionScript)