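; Reflective mirror for the light mechanic: the player can pick it up or rotate it, and it emits light while illuminated.
; E collects an unplaced mirror into BP_Khris_LightMechanic's count, or cycles yaw through looping MultiGate timeline turns.
; BP_LightTrigger_3B overlaps drive Activate and Deactivate, fading CylinderLight through a reversible timeline.
; Two interaction radii toggle arrow and prompt sprites, which yaw toward the camera every tick.
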(event OnComponentBeginOverlap(radius_interact2)
  (params (OverlappedComponent :type Primitive%20Component%20Object%20Reference) (OtherActor :type Actor%20Object%20Reference) (OtherComp :type Primitive%20Component%20Object%20Reference) (OtherBodyIndex :type Integer) (bFromSweep :type Boolean) (SweepResult :type Hit%20Result%20Structure%20%28by%20ref%29))
  ;[0.15 0.15 0.15 0.5] Interaction
  (bind _asbp_khris_light_mechanic (Utilities|Casting|CastToBP_Khris_LightMechanic OtherActor))
  (if (!= (Variables|/Game/ThirdPerson/Blueprints/BP_Khris_LightMechanic.BP_Khris_LightMechanic_C|GetLightCollision _asbp_khris_light_mechanic) OtherComp)
    (Development|SetHiddeninGame (Variables|Default|Getsolo_flecha_Sprite) false false)))

(event OnComponentEndOverlap(radius_interact)
  (params (OverlappedComponent :type Primitive%20Component%20Object%20Reference) (OtherActor :type Actor%20Object%20Reference) (OtherComp :type Primitive%20Component%20Object%20Reference) (OtherBodyIndex :type Integer))
  ;[0.15 0.15 0.15 0.5] Interaction
  (bind _asbp_khris_light_mechanic (Utilities|Casting|CastToBP_Khris_LightMechanic OtherActor))
  (if (!= (Variables|/Game/ThirdPerson/Blueprints/BP_Khris_LightMechanic.BP_Khris_LightMechanic_C|GetLightCollision _asbp_khris_light_mechanic) OtherComp)
    (Development|SetHiddeninGame (Variables|Default|GetUI_interacción+flecha_Sprite) true false)
    (Development|SetHiddeninGame (Variables|Default|Getsolo_flecha_Sprite) false false)
    (Variables|Default|SetCan%20rotate? false)
    (Variables|Default|SetCan%20Pick%20Mirror? false)))

(event OnComponentBeginOverlap(radius_interact)
  (params (OverlappedComponent :type Primitive%20Component%20Object%20Reference) (OtherActor :type Actor%20Object%20Reference) (OtherComp :type Primitive%20Component%20Object%20Reference) (OtherBodyIndex :type Integer) (bFromSweep :type Boolean) (SweepResult :type Hit%20Result%20Structure%20%28by%20ref%29))
  ;[0.15 0.15 0.15 0.5] Interaction
  (bind _asbp_khris_light_mechanic (Utilities|Casting|CastToBP_Khris_LightMechanic OtherActor))
  (if (!= (Variables|/Game/ThirdPerson/Blueprints/BP_Khris_LightMechanic.BP_Khris_LightMechanic_C|GetLightCollision _asbp_khris_light_mechanic) OtherComp)
    (Development|SetHiddeninGame (Variables|Default|GetUI_interacción+flecha_Sprite) false false)
    (Development|SetHiddeninGame (Variables|Default|Getsolo_flecha_Sprite) true false)
    (if (Variables|Default|GetIsMirrorPlaced?)
      (Variables|Default|SetCan%20rotate? true)
      (Variables|Default|SetCan%20Pick%20Mirror? false)
      (else
        (Variables|Default|SetCan%20rotate? true)
        (Variables|Default|SetCan%20Pick%20Mirror? true)))))

(event OnComponentEndOverlap(SphereCollision)
  (params (OverlappedComponent :type Primitive%20Component%20Object%20Reference) (OtherActor :type Actor%20Object%20Reference) (OtherComp :type Primitive%20Component%20Object%20Reference) (OtherBodyIndex :type Integer))
  ;[0.15 0.15 0.15 0.5] Controle whether the player is illuminating this object or not
  (Utilities|Casting|CastToBP_LightTrigger_3B OtherActor)
  (if true
    (Variables|Default|SetIlluminated false)
    (Development|PrintString "--- NOT ILLUMINATED")
    ;[0.15 0.15 0.15 0.5] Controls whether the object should acticate or not
    (if (Variables|Default|GetIlluminated)
      (CallFunction|Activate)
      (else
        (CallFunction|Deactivate)))))

(event OnComponentEndOverlap(radius_interact2)
  (params (OverlappedComponent :type Primitive%20Component%20Object%20Reference) (OtherActor :type Actor%20Object%20Reference) (OtherComp :type Primitive%20Component%20Object%20Reference) (OtherBodyIndex :type Integer))
  ;[0.15 0.15 0.15 0.5] Interaction
  (bind _asbp_khris_light_mechanic (Utilities|Casting|CastToBP_Khris_LightMechanic OtherActor))
  (if (!= (Variables|/Game/ThirdPerson/Blueprints/BP_Khris_LightMechanic.BP_Khris_LightMechanic_C|GetLightCollision _asbp_khris_light_mechanic) OtherComp)
    (Development|SetHiddeninGame (Variables|Default|Getsolo_flecha_Sprite) true false)))

(event OnComponentBeginOverlap(SphereCollision)
  (params (OverlappedComponent :type Primitive%20Component%20Object%20Reference) (OtherActor :type Actor%20Object%20Reference) (OtherComp :type Primitive%20Component%20Object%20Reference) (OtherBodyIndex :type Integer) (bFromSweep :type Boolean) (SweepResult :type Hit%20Result%20Structure%20%28by%20ref%29))
  ;[0.15 0.15 0.15 0.5] Controle whether the player is illuminating this object or not
  (Utilities|Casting|CastToBP_LightTrigger_3B OtherActor)
  (Variables|Default|SetIlluminated true)
  (Development|PrintString "--- ILLUMINATED")
  ;[0.15 0.15 0.15 0.5] Controls whether the object should acticate or not
  (if (Variables|Default|GetIlluminated)
    (CallFunction|Activate)
    (else
      (CallFunction|Deactivate))))

(event Custom|Activate
  ;[0.15 0.15 0.15 0.5] Light contorls (brighten and dim)
  (Variables|Default|SetActivated true)
  (Development|PrintString "--- ACTIVATED")
  (bind _intensity (Timeline|Timeline Play)
    (:Update
      (Rendering|Components|Light|SetIntensity (Variables|Default|GetCylinderLight) (Math|Float|Lerp 0.0 5e+03 _intensity))
      (Rendering|SetVisibility (Variables|Default|GetFlashlightFX) true false))))

(event Custom|Deactivate
  ;[0.15 0.15 0.15 0.5] Light contorls (brighten and dim)
  (Variables|Default|SetActivated false)
  (Development|PrintString "--- DEACTIVATED")
  (bind _intensity (Timeline|Timeline Reverse)
    (:Update
      (Rendering|Components|Light|SetIntensity (Variables|Default|GetCylinderLight) (Math|Float|Lerp 0.0 5e+03 _intensity))
      (Rendering|SetVisibility (Variables|Default|GetFlashlightFX) true false))))

(event EventTick
  (params (DeltaSeconds :type Float%20%28single-precision%29))
  ;[0.15 0.15 0.15 0.5] UI Interact always look front
  (Transformation|SetWorldRotation (Variables|Default|GetUI_interacción+flecha_Sprite) (Math|Rotator|MakeRotator 0.0 0.0 (.Yaw (Math|Rotator|BreakRotator (Math|Rotator|CombineRotators (Math|Rotator|FindLookatRotation (Transformation|GetWorldLocation (Variables|Default|Getsolo_flecha_Sprite)) (Camera|GetCameraLocation (Game|GetPlayerCameraManager 0))) "0.000000,-90.000000,0.000000")))) false false))

(event Input|KeyboardEvents|E
  (params (Key :type Key%20Structure :default "None"))
  ;[0.15 0.15 0.15 0.5] Agarrar objeto
  (:Pressed
    (if (not (Variables|Default|GetIsMirrorPlaced?))
      (if (Variables|Default|GetCan%20Pick%20Mirror?)
        (Utilities|FlowControl|DoOnce false
          (:Completed
            (bind _asbp_khris_light_mechanic (Utilities|Casting|CastToBP_Khris_LightMechanic (Game|GetPlayerCharacter 0)))
            (Variables|/Game/ThirdPerson/Blueprints/BP_Khris_LightMechanic.BP_Khris_LightMechanic_C|Setmirror? _asbp_khris_light_mechanic (+ (Variables|/Game/ThirdPerson/Blueprints/BP_Khris_LightMechanic.BP_Khris_LightMechanic_C|Getmirror? _asbp_khris_light_mechanic) 1))
            (bind _output_get (Variables|/Game/ThirdPerson/Blueprints/BP_Khris_LightMechanic.BP_Khris_LightMechanic_C|SetScale%20Mirror%20Saved _asbp_khris_light_mechanic (Transformation|GetWorldScale (Variables|Default|GetMirror_support))))
            (Transformation|SetWorldScale3D (Variables|Default|GetMirror) _output_get)
            (Actor|DestroyActor)
            (bind _returnvalue (UserInterface|CreateWidget "/Game/ui_ux/inventory/mirror_ui.mirror_ui_C"))
            (UserInterface|Viewport|AddtoViewport _returnvalue 0)
            (Utilities|FlowControl|Delay 3.0)
            (Widget|RemovefromParent _returnvalue)
            (Variables|Default|SetCan%20Pick%20Mirror? false)))))))

(event Input|KeyboardEvents|E
  (params (Key :type Key%20Structure :default "None"))
  ;[0.15 0.15 0.15 0.5] Press E to rotate
  (:Pressed
    (if (Variables|Default|GetCan%20rotate?)
      (if (not (Variables|Default|GetCan%20Pick%20Mirror?))
        (Utilities|Casting|CastToBP_Khris_LightMechanic (Game|GetPlayerCharacter 0))
        (Utilities|FlowControl|MultiGate false true -1
          (:Out%200
            (Variables|Default|SetSpin_Start 4e+01)
            (Variables|Default|SetSpin_End 0.0)
            (bind _movimiento (Timeline|Timeline_0 PlayFromStart)
              (:Update
                (Transformation|SetActorRotation (Math|Rotator|MakeRotator 0.0 0.0 (Math|Float|Lerp (Variables|Default|GetSpin_Start) (Variables|Default|GetSpin_End) _movimiento)))
                (Variables|Default|SetCan%20Pick%20Mirror? false))))
          (:Out%201
            (Variables|Default|SetSpin_Start 0.0)
            (Variables|Default|SetSpin_End -6e+01)
            (Timeline|Timeline_0 PlayFromStart))
          (:Out%202
            (Variables|Default|SetSpin_Start -6e+01)
            (Variables|Default|SetSpin_End 0.0)
            (Timeline|Timeline_0 PlayFromStart))
          (:Out%203
            (Variables|Default|SetSpin_Start 0.0)
            (Variables|Default|SetSpin_End 4e+01)
            (Timeline|Timeline_0 PlayFromStart)))))))

(fn ConstructionScript)

(fn IsPlayerIlluminated
  (bind _asbp_khris_light_mechanic (Utilities|Casting|CastToBP_Khris_LightMechanic (Game|GetPlayerCharacter 0))
    (:then
      (return (Variables|/Game/ThirdPerson/Blueprints/BP_Khris_LightMechanic.BP_Khris_LightMechanic_C|GetEstaIluminada _asbp_khris_light_mechanic)))
    (:CastFailed
      (return false))))